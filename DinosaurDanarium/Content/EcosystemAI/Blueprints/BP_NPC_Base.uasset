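; Base NPC animal Blueprint for an ecosystem simulation, handling needs, growth, breeding, attacking and death.
; A timed loop decays hunger, thirst and stamina, raises mating urge, and writes need flags to the AI blackboard.
; Animals ready to mate pair with opposite-gender members of their species, and females spawn scaled-down babies linked to their mother, within a population cap.
; An attack sphere-trace heavily damages other classes and refills food; zero health triggers ragdoll and timed removal.
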(event `self.ReceiveBeginPlay`
  ;[0 0 0] Begin Play
  (`self.Handle animal growth`)
  (`self.Update stats`)
  (`self.Update state`)
  (`BlackboardComponent.SetValueAsBool` (`AIBlueprintHelperLibrary.GetBlackboard` (`self.GetController`)) "IsPredator?" (select `/Game/EcosystemAI/Blueprints/Configuration/Enum_Diet` (`self.Diet`) :`NewEnumerator0` true))
  (`self.Check death`)
  ;[1 0 0.7825] (Debug) Init debug widget
  (bind _asaidebug_widget (cast `/Game/EcosystemAI/Blueprints/UI/AIDebugWidget` (`WidgetComponent.GetUserWidgetObject` (`self.DebugWidget`))))
  (set `/Game/EcosystemAI/Blueprints/UI/AIDebugWidget.Parent` self _asaidebug_widget))

(event `Update stats`
  (bind _stamina (`self.Stamina`))
  (bind _stamina_2 (`self.Stamina`))
  (bind _returnvalue (`AIBlueprintHelperLibrary.GetBlackboard` (`self.GetController`)))
  ;[0 0 0] Update stats
  (if (not (<= (`self.Health`) 0.0))
    (`|ExecutionSequence`
      (:`then_0`
        (`/Engine/EditorBlueprintResources/StandardMacros.DoOnce` false ; Skip delay the first time
          (:`Completed`
            _)))
      (:`then_1`
        (`KismetSystemLibrary.Delay` (`self.Seconds to update stats`))))
    (`self.Update stats`)
    (`|ExecutionSequence`
      (:`then_0`
        ;[0 0 0] Only decrease stats after splitting from mother
        (if (> (`self.Age`) 0.99)
          ;[0 0 0] Stat Decay
          ;;[0 0 0] Hunger decay
          (set `self.Food` (`KismetMathLibrary.FClamp` (- (`self.Food`) (`self.Hunger decay per update`)) 0.0 100.0))
          ;;[0 0 0] Thirst decay
          (set `self.Water` (`KismetMathLibrary.FClamp` (- (`self.Water`) (`self.Thirst decay per update`)) 0.0 100.0))
          ;;[0 0 0] Stamina decay
          (set `self.Stamina` (`KismetMathLibrary.FClamp` (`KismetMathLibrary.SelectFloat` (+ _stamina_2 (`self.Stamina refresh per update`)) (- _stamina_2 (`self.Stamina decay per update`)) (`self.Sleeping`)) 0.0 100.0))
          ;;[0 0 0] Mating urge refresh
          (set `self.Mating Urge` (`KismetMathLibrary.FClamp` (+ (`self.Mating Urge refresh per update`) (`self.Mating Urge`)) 0.0 100.0))
          ;[0 0 0] Health decay
          (if (`self.Should health decay if stats are low?`)
            (if (or (<= (`self.Water`) 1.0) (<= (`self.Food`) 1.0))
              (set `self.Health` (- (`self.Health`) (`self.Health decay per update`)))))))
      (:`then_1`
        ;[0 0 0] Update state
        (`BlackboardComponent.SetValueAsBool` _returnvalue "Hungry?" (< (`self.Food`) 30.0) :!label _label)
        (`BlackboardComponent.SetValueAsBool` _returnvalue "Thirsty?" (< (`self.Water`) 30.0))
        (`BlackboardComponent.SetValueAsBool` _returnvalue "Tired?" (select `bool` (`self.Sleeping`) :`false` (< _stamina 30.0) :`true` (< _stamina 99.0)))
        (`BlackboardComponent.SetValueAsBool` (`AIBlueprintHelperLibrary.GetBlackboard` (`self.GetController`)) "IsBaby?" (< (`self.Age`) 0.999))
        ;[0 0 0] Search for a partner
        (`/Engine/EditorBlueprintResources/StandardMacros.IsValid` (`self.Couple`)
          (:`Is Not Valid`
            (if (>= (`self.Mating Urge`) 99.0)
              (bind _outactors (`GameplayStatics.GetAllActorsOfClass` "BP_NPC_Base_C"))
              (for _array_element _outactors
                (if (and (== (`/Game/EcosystemAI/Blueprints/BP_NPC_Base.Species name` _array_element) (`self.Species name`)) (!= (`/Game/EcosystemAI/Blueprints/BP_NPC_Base.Gender` _array_element) (`self.Gender`)) (>= (`/Game/EcosystemAI/Blueprints/BP_NPC_Base.Mating Urge` _array_element) 99.900002) (not (`KismetSystemLibrary.IsValid` (`self.Couple`))) (> (`/Game/EcosystemAI/Blueprints/BP_NPC_Base.Health` _array_element) 0.01))
                  (`self.Set Couple` _array_element) ; Self
                  (`self.Set Couple` _array_element self) ; Other actor
                  (`self.Reset procreation`)
                  (`self.Reset procreation` _array_element)))))))
      (:`then_2`
        (`self.Check death`))
      (:`then_3`
        ;[1 0 0.9196] Cosmetic sleep particles
        (if (`self.Sleeping`)
          (`|ExecutionSequence`
            (:`then_0`
              (`/Engine/EditorBlueprintResources/StandardMacros.DoOnce` false
                (:`Completed`
                  (bind _returnvalue_2 (`AddComponent|NODE_AddParticleSystemComponent-0`)))))
            (:`then_1`
              (`ActorComponent.Activate` _returnvalue_2 false)))
          (else
            (`/Engine/EditorBlueprintResources/StandardMacros.IsValid` _returnvalue_2
              (:`Is Valid`
                (`ActorComponent.Deactivate` _returnvalue_2)))))))))

(event `Update state`
  ;[0 0 0] Update state
  (goto _label))

(event `Set Couple`
  (params (`Couple actor` :type "/Game/EcosystemAI/Blueprints/BP_NPC_Base Object Reference"))
  ;[0 0 0] Set couple
  (bind _output_get (set `self.Couple` `Couple actor`))
  (`BlackboardComponent.SetValueAsObject` (`AIBlueprintHelperLibrary.GetBlackboard` (`self.GetController`)) "Couple" _output_get))

(event `Handle animal growth`
  ;[0 0 0] Growth & Age
  (`TimelineComponent.SetPlayRate` (`self.Growth`) (/ 1.0 (`self.Growth time`)))
  (`|ExecutionSequence`
    (:`then_0`
      (bind (_direction _newtrack_0) (`Timeline|Growth` :`NewTime` (`self.Age`) :!via `SetNewTime` :!label _label_2)
        (:`Update`
          (set `self.Age` _newtrack_0)
          (`self.SetActorScale3D` (`KismetMathLibrary.Conv_DoubleToVector` (`KismetMathLibrary.Lerp` (`self.Baby actor scale`) 1.0 _newtrack_0))))))
    (:`then_1`
      (goto _label_2))))

(event `Have baby`
  (bind (_lowerbound _upperbound) (break `Int32Range` (`self.Babies per litter`)))
  (bind _returnvalue (`KismetMathLibrary.RandomIntegerInRange` (`.Value` (break `Int32RangeBound` _lowerbound)) (`.Value` (break `Int32RangeBound` _upperbound))))
  ;[0 0 0] Procreation
  (`/Engine/EditorBlueprintResources/StandardMacros.DoOnce` false :!label _label
    (:`Completed`
      (bind _outactors (`GameplayStatics.GetAllActorsOfClass` (`GameplayStatics.GetObjectClass` self)))
      (if (< (+ (`KismetArrayLibrary.Array_Length` _outactors) _returnvalue) (`self.Max world population`))
        (for _ (range 1 (+ _returnvalue 1))
          (set `self.Mating Urge` 0.0)
          (switch `/Game/EcosystemAI/Blueprints/Configuration/Enum_Gender` (`self.Gender`)
            (:`NewEnumerator1`
              (`/Engine/EditorBlueprintResources/StandardMacros.IsValid` self
                (:`Is Valid`
                  (bind _returnvalue_2 (`|SpawnActorFromClass` (`GameplayStatics.GetObjectClass` self) (`self.GetTransform`) "Undefined" "OverrideRootScale" null 0.001 true "NewEnumerator0" null))
                  (if (and (`KismetSystemLibrary.IsValid` self) (`KismetSystemLibrary.IsValid` _returnvalue_2))
                    (set `/Game/EcosystemAI/Blueprints/BP_NPC_Base.Mother` self _returnvalue_2)
                    (`BlackboardComponent.SetValueAsObject` (`AIBlueprintHelperLibrary.GetBlackboard` (`self.GetController` _returnvalue_2)) "Mother" self)
                    ;[1 0 0.926] Display particles
                    (`GameplayStatics.SpawnEmitterAtLocation` "/Game/EcosystemAI/Particles/PS_Love.PS_Love" (`self.K2_GetActorLocation`))
                    (else
                      (`/Engine/EditorBlueprintResources/StandardMacros.IsValid` _returnvalue_2
                        (:`Is Valid`
                          (`self.K2_DestroyActor` _returnvalue_2))))))))))
        (else
          (set `self.Mating Urge` 0.0))))))

(event `Reset procreation`
  ;[0 0 0] Procreation
  (goto _label :!via `Reset`))

(event `Check death`
  ;[0 0 0] Death
  (if (<= (stale `self.ReceiveAnyDamage` _output_get) 0.0) :!label _label_2
    (`PrimitiveComponent.SetSimulatePhysics` (`self.Mesh`) true)
    (`PrimitiveComponent.SetCollisionEnabled` (`self.CapsuleComponent`) "NoCollision")
    (`CharacterMovementComponent.DisableMovement` (`self.CharacterMovement`))
    (`PrimitiveComponent.SetCollisionEnabled` (`self.Mesh`) "QueryAndPhysics")
    (`self.SetLifeSpan` 25.0)))

(event `self.ReceiveAnyDamage`
  (params (Damage :type "Float (single-precision)") (DamageType :type "DamageType Object Reference") (InstigatedBy :type "Controller Object Reference") (DamageCauser :type "Actor Object Reference"))
  ;[0 0 0] Death
  (bind _output_get (set `self.Health` (- (`self.Health`) Damage)))
  (goto _label_2))

(event `Attack`
  (bind _returnvalue (`self.K2_GetActorLocation`))
  ;[0 0 0] Attack
  (bind (_outhit _returnvalue_2) (`KismetSystemLibrary.SphereTraceSingleForObjects` _returnvalue _returnvalue 300.0 (`|MakeArray` "ObjectTypeQuery3" :!type "EObjectTypeQuery Enum")))
  (if _returnvalue_2
    (bind (_bblockinghit _binitialoverlap _time _distance _location _impactpoint _normal _impactnormal _physmat _hitactor) (`GameplayStatics.BreakHitResult` _outhit))
    (if (not (== (`GameplayStatics.GetObjectClass` _hitactor) (`GameplayStatics.GetObjectClass` self)))
      (`GameplayStatics.ApplyDamage` _hitactor 555.0)
      (set `self.Food` 100.0)
      (`self.PlayAnimMontage` (`self.Attack anim montage`)))))

(fn `UserConstructionScript`
  (set `CharacterMovementComponent.MaxWalkSpeed` (`self.Max walk speed`) (`self.CharacterMovement`))
  (if (`self.Randomize Gender?`)
    (set `self.Gender` (select `bool` (`KismetMathLibrary.RandomBool`) :`false` "NewEnumerator0" :`true` "NewEnumerator1" :!type "/Game/EcosystemAI/Blueprints/Configuration/Enum_Gender Enum"))))