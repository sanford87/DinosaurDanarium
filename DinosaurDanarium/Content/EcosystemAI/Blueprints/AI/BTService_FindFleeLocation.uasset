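; Behavior tree service that gives an Ecosystem AI NPC a location to flee to from nearby predators.
; On activation it caches the controlled NPC, then each tick scans all BP_NPC_Base actors for carnivores within detection distance.
; For a match it writes a random reachable point, around a spot offset away from that predator, to the "Target Location" blackboard key.
; The loop has no break, so the last matching predator wins.
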(event `self.ReceiveTickAI`
  (params (OwnerController :type "AIController Object Reference") (ControlledPawn :type "Pawn Object Reference") (DeltaSeconds :type "Float (single-precision)"))
  (bind _outactors (`GameplayStatics.GetAllActorsOfClass` "/Game/EcosystemAI/Blueprints/BP_NPC_Base.BP_NPC_Base_C"))
  (for _array_element _outactors
    (`/Engine/EditorBlueprintResources/StandardMacros.IsValid` _array_element
      (:`Is Valid`
        (if (and (select `/Game/EcosystemAI/Blueprints/Configuration/Enum_Diet` (`/Game/EcosystemAI/Blueprints/BP_NPC_Base.Diet` _array_element) :`NewEnumerator0` true) (< (`Actor.GetDistanceTo` _array_element (stale `self.ReceiveActivationAI` _asbp_npc_base)) (`self.Distance to find enemy`)) (`KismetSystemLibrary.IsValid` _array_element) (`KismetSystemLibrary.IsValid` (stale `self.ReceiveActivationAI` _asbp_npc_base)))
          (bind _returnvalue (`Actor.K2_GetActorLocation` (stale `self.ReceiveActivationAI` _asbp_npc_base)))
          (`BlackboardComponent.SetValueAsVector` (`AIBlueprintHelperLibrary.GetBlackboard` OwnerController) "Target Location" (`NavigationSystemV1.K2_GetRandomReachablePointInRadius` (+ _returnvalue (* (`KismetMathLibrary.GetForwardVector` (`KismetMathLibrary.FindLookAtRotation` _returnvalue (`Actor.K2_GetActorLocation` _array_element))) -100.0)) 150.0 null null)))))))

(event `self.ReceiveActivationAI`
  (params (OwnerController :type "AIController Object Reference") (ControlledPawn :type "Pawn Object Reference"))
  ;[0 0 0] Get  controlled NPC
  (bind _asbp_npc_base (cast `/Game/EcosystemAI/Blueprints/BP_NPC_Base` ControlledPawn)))