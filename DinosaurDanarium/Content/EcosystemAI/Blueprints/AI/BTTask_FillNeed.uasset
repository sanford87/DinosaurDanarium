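; Behavior tree task that refills one basic need, water or food, on an NPC in the ecosystem AI.
; It sets the chosen stat on the controlled BP_NPC_Base to full, updates its stats and flags it as filling needs.
; It then clears the matching Thirsty or Hungry blackboard bool and finishes successfully in the same execution.
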(event `self.ReceiveExecuteAI`
  (params (OwnerController :type "AIController Object Reference") (ControlledPawn :type "Pawn Object Reference"))
  (bind _basic_need_to_fill (`self.Basic need to fill`))
  (bind _asbp_npc_base (cast `/Game/EcosystemAI/Blueprints/BP_NPC_Base` ControlledPawn))
  (switch `/Game/EcosystemAI/Blueprints/Configuration/Enum_BasicNeeds` _basic_need_to_fill
    (:`NewEnumerator0`
      (set `/Game/EcosystemAI/Blueprints/BP_NPC_Base.Water` 100.0 _asbp_npc_base))
    (:`NewEnumerator1`
      (set `/Game/EcosystemAI/Blueprints/BP_NPC_Base.Food` 100.0 _asbp_npc_base)))
  (`/Game/EcosystemAI/Blueprints/BP_NPC_Base.Update stats` _asbp_npc_base)
  (set `/Game/EcosystemAI/Blueprints/BP_NPC_Base.Filling needs` true _asbp_npc_base)
  (`BlackboardComponent.SetValueAsBool` (`AIController.Blackboard` OwnerController) (select `/Game/EcosystemAI/Blueprints/Configuration/Enum_BasicNeeds` _basic_need_to_fill :`NewEnumerator0` "Thirsty?" :`NewEnumerator1` "Hungry?") false)
  (`self.FinishExecute` true))