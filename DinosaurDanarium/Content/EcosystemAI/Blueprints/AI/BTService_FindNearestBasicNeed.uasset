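; Behavior tree service that points an AI pawn at the nearest water or food source, depending on its SearchFor setting.
; When the tree search starts, it loops over all actors of that source class, keeping a running minimum distance from the pawn.
; Each closer source overwrites the blackboard's Target Location with a random reachable point within its root component's bounds radius, if one is found.
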(event `self.ReceiveSearchStartAI`
  (params (OwnerController :type "AIController Object Reference") (ControlledPawn :type "Pawn Object Reference"))
  (bind _search_for (`self.Search for`))
  (set `self.Nearest Distance` 999999995904.0)
  (switch `/Game/EcosystemAI/Blueprints/Configuration/Enum_BasicNeeds` _search_for
    (:`NewEnumerator0`
      (bind _outactors (`GameplayStatics.GetAllActorsOfClass` "/Game/EcosystemAI/Blueprints/BP_WaterSource.BP_WaterSource_C"))
      (for _array_element _outactors
        (`self.Is Nearest Actor?` _array_element ControlledPawn
          (:`True`
            (bind _returnvalue (select `/Game/EcosystemAI/Blueprints/Configuration/Enum_BasicNeeds` _search_for :`NewEnumerator0` _array_element :`NewEnumerator1` (stale _array_element_2) :!type "Actor Object Reference"))
            (`/Engine/EditorBlueprintResources/StandardMacros.IsValid` _returnvalue :!label _label
              (:`Is Valid`
                (bind (_randomlocation _returnvalue_2) (`NavigationSystemV1.K2_GetRandomReachablePointInRadius` (`Actor.K2_GetActorLocation` _returnvalue) (`.SphereRadius` (`KismetSystemLibrary.GetComponentBounds` (`Actor.RootComponent` _returnvalue))) null null))
                (if _returnvalue_2
                  (`BlackboardComponent.SetValueAsVector` (`AIBlueprintHelperLibrary.GetBlackboard` OwnerController) "Target Location" _randomlocation))))))))
    (:`NewEnumerator1`
      (bind _outactors_2 (`GameplayStatics.GetAllActorsOfClass` "/Game/EcosystemAI/Blueprints/BP_FoodSource.BP_FoodSource_C"))
      (for _array_element_2 _outactors_2
        (`self.Is Nearest Actor?` _array_element_2 ControlledPawn
          (:`True`
            (goto _label)))))))