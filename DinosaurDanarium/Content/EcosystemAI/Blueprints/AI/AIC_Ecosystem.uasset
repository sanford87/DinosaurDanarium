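; AI controller for ecosystem NPCs that runs the ecosystem behavior tree and picks an enemy from perceived actors.
; On perception updates, if the Blackboard has no valid Enemy, it scans currently perceived NPCs and stores the first qualifying one.
; A helper check qualifies a target as potential food or predator when it is alive, adult and has a different Diet from the controlled pawn.
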(event `self.AIPerception.OnPerceptionUpdated`
  (params (UpdatedActors :type "Array of Actor Object Reference (by ref)"))
  (bind _returnvalue (`AIBlueprintHelperLibrary.GetBlackboard` null))
  (`/Engine/EditorBlueprintResources/StandardMacros.IsValid` (`BlackboardComponent.GetValueAsObject` _returnvalue "Enemy")
    (:`Is Not Valid`
      (for _array_element (`AIPerceptionComponent.GetCurrentlyPerceivedActors` (`self.AIPerception`) null)
        (bind _asbp_npc_base (cast `/Game/EcosystemAI/Blueprints/BP_NPC_Base` _array_element))
        (bind _asbp_npc_base_2 (cast `/Game/EcosystemAI/Blueprints/BP_NPC_Base` (`self.K2_GetPawn`)))
        (if (and (`KismetSystemLibrary.IsValid` _asbp_npc_base) (not (<= (`/Game/EcosystemAI/Blueprints/BP_NPC_Base.Health` _asbp_npc_base) 0.0)) (== (`/Game/EcosystemAI/Blueprints/BP_NPC_Base.Age` _asbp_npc_base) 1.0) (!= (`/Game/EcosystemAI/Blueprints/BP_NPC_Base.Diet` _asbp_npc_base_2) (`/Game/EcosystemAI/Blueprints/BP_NPC_Base.Diet` _asbp_npc_base)))
          (`BlackboardComponent.SetValueAsObject` _returnvalue "Enemy" _asbp_npc_base)
          (break))))))

(event `self.ReceiveBeginPlay`
  (`self.RunBehaviorTree` "/Game/EcosystemAI/Blueprints/AI/BT_Ecosystem.BT_Ecosystem"))

(fn `UserConstructionScript`)